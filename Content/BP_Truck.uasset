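; BP_Truck is an actor that drives a Truck component along its spline.
; Each tick it copies speed from the PythonVel value on a Target reference and accumulates distance travelled.
; It sets the truck's relative transform from the spline's local transform at that distance, with a -90 degree yaw offset, and stores the X and Y position.
; When Loop is enabled, distance resets to zero past the spline's end.
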(event EventTick
  (params (DeltaSeconds :type Float%20%28single-precision%29))
  (Variables|Default|SetSpeed (Variables|/Game/PythonScript.PythonScript_C|GetPythonVel (Variables|Default|GetTarget)))
  (Variables|Default|SetDistance (+ (* DeltaSeconds (Variables|Default|GetSpeed)) (Variables|Default|GetDistance)))
  (Variables|Default|SetPos_X (.x (.location (Spline|GetTransformatDistanceAlongSpline (Variables|Default|GetSpline) (Variables|Default|GetDistance) "Local" false))))
  (Variables|Default|SetPos_Y (.y (.location (Spline|GetTransformatDistanceAlongSpline (Variables|Default|GetSpline) (Variables|Default|GetDistance) "Local" false))))
  (Transformation|SetRelativeTransform (Variables|Default|GetTruck) (Math|Transform|MakeTransform (Math|Vector|MakeVector (.x (.location (Spline|GetTransformatDistanceAlongSpline (Variables|Default|GetSpline) (Variables|Default|GetDistance) "Local" false))) (.y (.location (Spline|GetTransformatDistanceAlongSpline (Variables|Default|GetSpline) (Variables|Default|GetDistance) "Local" false))) (.z (.location (Spline|GetTransformatDistanceAlongSpline (Variables|Default|GetSpline) (Variables|Default|GetDistance) "Local" false)))) (Math|Rotator|MakeRotator (.roll (.rotation (Spline|GetTransformatDistanceAlongSpline (Variables|Default|GetSpline) (Variables|Default|GetDistance) "Local" false))) (.pitch (.rotation (Spline|GetTransformatDistanceAlongSpline (Variables|Default|GetSpline) (Variables|Default|GetDistance) "Local" false))) (+ (.yaw (.rotation (Spline|GetTransformatDistanceAlongSpline (Variables|Default|GetSpline) (Variables|Default|GetDistance) "Local" false))) -9e+01)) "1.000000,1.000000,1.000000") false false)
  (if (Variables|Default|GetLoop)
    (if (> (Variables|Default|GetDistance) (Spline|GetSplineLength (Variables|Default|GetSpline)))
      (Variables|Default|SetDistance 0.0))))

(fn ConstructionScript)